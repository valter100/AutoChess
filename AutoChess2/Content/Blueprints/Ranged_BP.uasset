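; Ranged_BP is a ranged unit Blueprint with an archer animation and an overhead health and mana bar.
; On BeginPlay it binds the bar widget component to itself and caches the WBP_Archer anim instance.
; Tick pushes the unit's moving and attacking states into that anim instance every frame.
; A separate CreateHealthBar function can spawn a viewport bar widget, though nothing in this file calls it.
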(event `self.ReceiveBeginPlay`
  (bind _aswb_unit_bars (cast `/Game/UI/WB_UnitBars` (`WidgetComponent.GetUserWidgetObject` (`self.HealthManaBar`))))
  (set `/Game/UI/WB_UnitBars.Unit` self _aswb_unit_bars)
  (bind _aswbp_archer (cast `/Game/ImportedAssets/Characters/Lite_Longbow_Pack/WBP_Archer` (`SkeletalMeshComponent.GetAnimInstance` (`self.CharacterMesh`))))
  (set `self.AnimationInstance` _aswbp_archer))

(event `self.ReceiveTick`
  (params (DeltaSeconds :type "Float (single-precision)"))
  (set `/Game/ImportedAssets/Characters/Lite_Longbow_Pack/WBP_Archer.IsWalking` (`self.GetIsMoving`) (`self.AnimationInstance`))
  (set `/Game/ImportedAssets/Characters/Lite_Longbow_Pack/WBP_Archer.IsAttacking` (`self.GetIsAttacking`) (`self.AnimationInstance`)))

(fn `CreateHealthBar`
  (bind _returnvalue (`|CreateWidget` "/Game/UI/WB_UnitBars.WB_UnitBars_C"))
  (`UserWidget.AddToViewport` _returnvalue 0)
  (set `/Game/UI/WB_UnitBars.Unit` self _returnvalue))

(fn `UserConstructionScript`)