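; Unit shop Blueprint that populates the shop's units and owns its on-screen UI.
; On BeginPlay it calls AddUnits, then creates a UnitShop_UI widget, hands it a self reference and adds it to the viewport.
; ToggleShopBP passes the NotVisible flag to the widget, flips it, and calls RefreshUnits whenever the flag becomes false.
; AddUnits and RefreshUnits are not defined in this graph.
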(event `self.ReceiveBeginPlay`
  (`self.AddUnits`)
  (bind _returnvalue (`|CreateWidget` "/Game/UI/UnitShop_UI.UnitShop_UI_C"))
  (`/Game/UI/UnitShop_UI.SetUnitShop` _returnvalue self)
  (`UserWidget.AddToViewport` _returnvalue 0)
  (set `self.Shop UI` _returnvalue))

(fn `ToggleShopBP`
  (bind _notvisible (`self.NotVisible`))
  (`/Game/UI/UnitShop_UI.ToggleShop` (`self.Shop UI`) _notvisible)
  (bind _output_get (set `self.NotVisible` (not _notvisible)))
  (if (not _output_get)
    (`self.RefreshUnits`)))

(fn `UserConstructionScript`)