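; RoundManager_BP is the round controller that alternates the game between a shop/placement phase and a battle phase on a shared timer.
; BeginPlay caches the shop, placer, node manager, player and opponent actors and creates the round UI.
; Tick drives NewRound, which toggles shop and placement, then either generates and activates opposing teams or cleans up and resets units.
; During battle, either side running out of units fast-forwards the timer to five seconds remaining.
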(event `self.ReceiveBeginPlay`
  (bind _outactors (`GameplayStatics.GetAllActorsOfClass` "/Game/Blueprints/UnitShop_BP.UnitShop_BP_C"))
  (set `self.UnitShop` (`|GetArrayItem` _outactors))
  (bind _returnvalue (`|CreateWidget` "/Game/UI/RoundManager_UI.RoundManager_UI_C"))
  (`/Game/UI/RoundManager_UI.SetRoundManagerBP` _returnvalue self)
  (`UserWidget.AddToViewport` _returnvalue 0)
  (bind _outactors_2 (`GameplayStatics.GetAllActorsOfClass` "/Game/Blueprints/UnitPlacer_BP.UnitPlacer_BP_C"))
  (set `self.UnitPlacer` (`|GetArrayItem` _outactors_2))
  (bind _outactors_3 (`GameplayStatics.GetAllActorsOfClass` "/Game/Blueprints/NodeManager_BP.NodeManager_BP_C"))
  (set `self.NodeManager` (`|GetArrayItem` _outactors_3))
  (bind _outactors_4 (`GameplayStatics.GetAllActorsOfClass` "/Script/AutoChess2.MyPlayer"))
  (set `self.Player` (`|GetArrayItem` _outactors_4))
  (bind _outactors_5 (`GameplayStatics.GetAllActorsOfClass` "/Game/Blueprints/MyOpponent_BP.MyOpponent_BP_C"))
  (set `self.Opponent` (`|GetArrayItem` _outactors_5))
  (`self.SetTimeBetweenRounds` 30.0))

(event `self.ReceiveTick`
  (params (DeltaSeconds :type "Float (single-precision)"))
  (bind _returnvalue (`self.GetTimeBetweenRounds`))
  (`self.SetRoundTimer` (+ (`self.GetRoundTimer`) DeltaSeconds))
  (if (>= (`self.GetRoundTimer`) (`self.GetTimeBetweenRounds`))
    (`self.NewRound`)
    (elif (`self.IsBattlePhase`)
      (if (and (and (`MyPlayer.HasRemainingUnitsOnBoard` (`self.Player`)) (`MyOpponent.HasRemainingUnitsOnBoard` (`self.Opponent`))) (>= _returnvalue 5.0))
        _
        (elif (not (`self.EarlySwapCalled`))
          (`self.SetRoundTimer` (- _returnvalue 5.0))
          (set `self.EarlySwapCalled` true))))))

(fn `NewRound`
  (bind _opponent (`self.Opponent`))
  (bind _player (`self.Player`))
  (bind _player_2 (`self.Player`))
  (bind _opponent_2 (`self.Opponent`))
  (`self.SetRoundTimer` 0.0)
  (set `self.IsBattlePhase` (not (`self.IsBattlePhase`)))
  (set `self.EarlySwapCalled` false)
  (`/Game/Blueprints/UnitShop_BP.ToggleShopBP` (`self.UnitShop`))
  (`/Game/Blueprints/UnitPlacer_BP.On Round Swap` (`self.UnitPlacer`))
  (`NodeManager.TogglePlacementNodes` (`self.NodeManager`))
  (if (`self.IsBattlePhase`)
    (`MyOpponent.GenerateTeam` _opponent)
    (`MyOpponent.ActivateUnits` _opponent)
    (`MyPlayer.ActivateUnits` _player)
    (`MyPlayer.SetOpponentUnits` _player_2 (`MyOpponent.GetSpawnedUnits` _opponent_2))
    (`MyOpponent.SetOpponentUnits` _opponent_2 (`MyPlayer.GetUnitsOnBoard` _player_2))
    (else
      (`MyOpponent.CleanUpUnits` _opponent)
      (`MyPlayer.ResetUnitsOnBoard` _player))))

(fn `UserConstructionScript`)