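; UnitPlacer_BP is a player-input actor that lets the player pick up, drop and sell units outside the battle phase.
; It finds the round manager and unit shop at BeginPlay.
; Left click either drops the held unit, selling it through the shop if its sell flag is set, or picks up the Unit hit by a cursor trace.
; A round swap releases any held unit.
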(event `self.ReceiveBeginPlay`
  (`self.EnableInput` (`GameplayStatics.GetPlayerController` 0))
  (bind _outactors (`GameplayStatics.GetAllActorsOfClass` "/Game/Blueprints/RoundManager_BP.RoundManager_BP_C"))
  (set `self.RoundManagerBP` (`|GetArrayItem` _outactors))
  (bind _outactors_2 (`GameplayStatics.GetAllActorsOfClass` "/Game/Blueprints/UnitShop_BP.UnitShop_BP_C"))
  (set `self.Unit Shop` (`|GetArrayItem` _outactors_2)))

(event `Key|LeftMouseButton`
  (params (Key :type "Key Structure"))
  (bind _returnvalue (`self.GetPickedUpUnit`))
  (bind _returnvalue_2 (`self.GetPickedUpUnit`))
  (:`Pressed`
    (if (`/Game/Blueprints/RoundManager_BP.IsBattlePhase` (`self.RoundManagerBP`))
      _
      (elif (`KismetSystemLibrary.IsValid` (`self.GetPickedUpUnit`))
        (`Unit.SetPickedUp` _returnvalue false)
        (if (`Unit.GetSell` _returnvalue)
          (`self.Sell Picked Up Unit`))
        (`self.SetPickedUpUnitToNull`)
        (else
          (bind _asunit (`self.Get Unit Under Cursor`))
          (`Unit.SetPickedUp` _asunit true)
          (`self.SetPickedUpUnit` _asunit)
          (if (`Unit.GetPickedUp` _returnvalue_2)
            _
            (elif (`Unit.GetSell` _returnvalue_2)
              (`UnitShop.SellUnit` (`self.Unit Shop`) null)
              (`self.SetPickedUpUnitToNull`))))))))

(event `On Round Swap`
  (bind _returnvalue (`self.GetPickedUpUnit`))
  (if (`KismetSystemLibrary.IsValid` _returnvalue)
    (`Unit.SetPickedUp` _returnvalue false)
    (`self.SetPickedUpUnitToNull`)))

(fn `Get Unit Under Cursor`
  (returns (AsUnit :type "Unit Object Reference"))
  (bind _asunit (cast `Unit` (`.HitActor` (`GameplayStatics.BreakHitResult` (`PlayerController.GetHitResultUnderCursorForObjects` (`GameplayStatics.GetPlayerController` 0) (`|MakeArray` "ObjectTypeQuery2" :!type "EObjectTypeQuery Enum") true))))
    (:`then`
      _)
    (:`CastFailed`
      _))
  (return _asunit))

(fn `Sell Picked Up Unit`
  (`UnitShop.SellUnit` (`self.Unit Shop`) (`self.GetPickedUpUnit`)))

(fn `UserConstructionScript`)